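; BP_Ball is a player-controlled physics ball that rolls around and aims a gun at the mouse cursor.
; Enhanced Input drives it, with move input applying an acceleration force to the damped sphere every tick.
; A BP_Gun spawned at BeginPlay attaches to the Gun component, whose absolute rotation ignores the roll and yaws toward a cursor line trace hit.
; Shooting calls Fire on that gun, throttled by a short cooldown.
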(event Input|EnhancedActionEvents|EnhancedInputActionIA_Move
  (params (ActionValue :type Vector%202D%20Structure) (ElapsedSeconds :type Float%20%28double-precision%29) (TriggeredSeconds :type Float%20%28double-precision%29) (InputAction :type Input%20Action%20Object%20Reference :default "/Game/Input/InputActions/IA_Move.IA_Move"))
  (:Triggered
    (Variables|Default|SetInputDirection ActionValue)
    (Variables|Default|SetbMoveActionTriggered true))
  (:Completed
    (Variables|Default|SetbMoveActionTriggered false)))

(event Input|EnhancedActionEvents|EnhancedInputActionIA_Shoot
  (params (ActionValue :type Boolean) (ElapsedSeconds :type Float%20%28double-precision%29) (TriggeredSeconds :type Float%20%28double-precision%29) (InputAction :type Input%20Action%20Object%20Reference :default "/Game/Input/InputActions/IA_Shoot.IA_Shoot"))
  (:Triggered
    (if (Variables|Default|GetbCanShoot)
      (Variables|Default|SetbCanShoot false)
      (Default|Fire (Variables|Default|GetBP_Gun))
      (Utilities|FlowControl|Delay 0.2)
      (Variables|Default|SetbCanShoot true))))

(event EventBeginPlay
  (bind _gun (Variables|Default|GetGun))
  (bind _gun_2 (Variables|Default|GetGun))
  (bind _sphere (Variables|Default|GetSphere))
  (bind _returnvalue (Transformation|GetWorldTransform _gun))
  (bind _asplayer_controller (Utilities|Casting|CastToPlayerController (Game|GetPlayerController 0)))
  (Utilities|IsValid (PlayerController|LocalPlayerSubsystems|GetEnhancedInputLocalPlayerSubsystem _asplayer_controller)
    (:Is%20Valid
      (Input|AddMappingContext (PlayerController|LocalPlayerSubsystems|GetEnhancedInputLocalPlayerSubsystem _asplayer_controller) "/Game/Input/IMC_DefaultInputMappingContext.IMC_DefaultInputMappingContext" 0 "(bIgnoreAllPressedKeysUntilRelease=True,bForceImmediately=False)")
      (Class|PrimitiveComponent|SetLinearDamping _sphere 1.5)
      (Class|PrimitiveComponent|SetAngularDamping _sphere 0.0)
      (Transformation|SetAbsolute (Variables|Default|GetGun) false true false)
      (bind _returnvalue_2 (Game|SpawnActorfromClass "/Game/_Game/Blueprints/Guns/BP_Gun.BP_Gun_C" (Math|Transform|MakeTransform (.location _returnvalue) (.rotation _returnvalue) "1.000000,1.000000,1.000000") "AdjustIfPossibleButAlwaysSpawn" 0 0))
      (bind _output_get (Variables|Default|SetBP_Gun _returnvalue_2))
      (Transformation|AttachComponentToComponent _output_get _gun_2 "None" "SnapToTarget" "KeepWorld" "KeepWorld" false)
      (Collision|SetCollisionEnabled _gun_2 "QueryAndPhysics"))))

(event EventTick
  (params (DeltaSeconds :type Float%20%28single-precision%29))
  (bind _impactpoint (CallFunction|LineTraceforBodyRotation))
  (Transformation|SetWorldRotation (Variables|Default|GetGun) (Math|Rotator|MakeRotator 0.0 0.0 (.yaw (Math|Rotator|FindLookatRotation (Transformation|GetWorldLocation (Variables|Default|GetGun)) _impactpoint))) false false)
  (if (Variables|Default|GetbMoveActionTriggered)
    (Physics|AddForce (Variables|Default|GetSphere) (CallFunction|GetMovementForceDirection) "None" true)))

(fn ConstructionScript)

(fn GetMovementForceDirection
  (bind _moveforce (Variables|Default|GetMoveForce))
  (return (Math|Conversions|ToVector(Vector2D) (* (Variables|Default|GetInputDirection) (Math|Vector2D|MakeVector2D _moveforce _moveforce)))))

(fn LineTraceforBodyRotation
  (bind _returnvalue (Game|GetPlayerController 0))
  (bind (_worldlocation _worlddirection) (Game|Player|ConvertMouseLocationToWorldSpace _returnvalue))
  (bind _outhit (Collision|LineTraceByChannel _worldlocation (+ _worldlocation (* _worlddirection 5e+03)) "TraceTypeQuery1" false 0 "None"))
  (return (.ImpactPoint (Collision|BreakHitResult _outhit))))