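; Test player-controlled mech that toggles between a physics-driven ball form and a walking mech form when X is pressed.
; Enhanced Input stores the move direction, and Tick applies the current form's capsule size and physics state every frame.
; Ball form pushes the simulated capsule with acceleration-based force, while mech form disables physics and uses movement input along X only.
; The PlayAnimation flag doubles as the form switch.
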(event Input|EnhancedActionEvents|EnhancedInputActionIA_Move
  (params (ActionValue :type Vector%202D%20Structure) (ElapsedSeconds :type Float%20%28double-precision%29) (TriggeredSeconds :type Float%20%28double-precision%29) (InputAction :type Input%20Action%20Object%20Reference :default "/Game/Input/InputActions/IA_Move.IA_Move"))
  (:Triggered
    (Variables|Default|SetInputDirection ActionValue)
    (Variables|Default|SetbMove true))
  (:Completed
    (Variables|Default|SetbMove false)))

(event EventBeginPlay
  (bind _returnvalue (Game|GetPlayerController 0))
  (bind _returnvalue_2 (PlayerController|LocalPlayerSubsystems|GetEnhancedInputLocalPlayerSubsystem _returnvalue))
  (Utilities|IsValid _returnvalue_2
    (:Is%20Valid
      (Input|AddMappingContext _returnvalue_2 "/Game/Input/IMC_DefaultInputMappingContext.IMC_DefaultInputMappingContext" 0 "(bIgnoreAllPressedKeysUntilRelease=True,bForceImmediately=False)"))))

(event EventTick
  (params (DeltaSeconds :type Float%20%28single-precision%29))
  (bind _inputdirection (Variables|Default|GetInputDirection))
  (bind _inputdirection_2 (Variables|Default|GetInputDirection))
  (bind _capsule (Variables|Default|GetCapsule))
  (bind _capsule_2 (Variables|Default|GetCapsule))
  (if (not (Variables|Default|GetPlayAnimation))
    (Physics|SetSimulatePhysics (Variables|Default|GetCapsule) true)
    (Components|Capsule|SetCapsuleHalfHeight _capsule_2 (Variables|Default|GetCapsuleHeightBall) true)
    (Components|Capsule|SetCapsuleRadius _capsule_2 (Variables|Default|GetCapsuleRadiusBall) true)
    (if (Variables|Default|GetbMove)
      (Physics|AddForce (Variables|Default|GetCapsule) (Math|Vector|MakeVector (* (Variables|Default|GetForce) (.x _inputdirection_2) -1.0) (* (.y _inputdirection_2) (Variables|Default|GetForce)) 0.0) "None" true))
    (else
      (Physics|SetSimulatePhysics (Variables|Default|GetCapsule) false)
      (Components|Capsule|SetCapsuleHalfHeight _capsule (Variables|Default|GetCapsuleHeightMech) true)
      (Components|Capsule|SetCapsuleRadius _capsule (Variables|Default|GetCapsuleRadiusMech) true)
      (if (Variables|Default|GetbMove)
        (Pawn|Input|AddMovementInput (Math|Vector|MakeVector (* (Variables|Default|GetForce) (.x _inputdirection) -1.0) (* (.y _inputdirection) 0.0) 0.0) 1.0 true)))))

(event Input|KeyboardEvents|X
  (params (Key :type Key%20Structure))
  (:Pressed
    (Variables|Default|SetPlayAnimation (not (Variables|Default|GetPlayAnimation)))))

(fn ConstructionScript)