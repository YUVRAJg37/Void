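; Player-controlled ball character that rolls on a physics-driven lower body while its upper body and gun aim at the mouse cursor.
; Enhanced Input movement applies torque each tick, plus a turning force that grows as input opposes velocity unless ForceOverride is set.
; A cursor line trace sets upper body and gun yaw.
; A BP_GunTest spawned on BeginPlay attaches to the gun and fires on a short cooldown.
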(event Input|EnhancedActionEvents|EnhancedInputActionIA_Move
  (params (ActionValue :type Vector%202D%20Structure) (ElapsedSeconds :type Float%20%28double-precision%29) (TriggeredSeconds :type Float%20%28double-precision%29) (InputAction :type Input%20Action%20Object%20Reference :default "/Game/Input/InputActions/IA_Move.IA_Move"))
  ;[1 1 1] Movement Action
  (:Triggered
    (Variables|Default|SetInputDirection ActionValue)
    (Variables|Default|SetbMoveActionTriggered true))
  (:Completed
    (Variables|Default|SetbMoveActionTriggered false)))

(event Input|EnhancedActionEvents|EnhancedInputActionIA_Shoot
  (params (ActionValue :type Boolean) (ElapsedSeconds :type Float%20%28double-precision%29) (TriggeredSeconds :type Float%20%28double-precision%29) (InputAction :type Input%20Action%20Object%20Reference :default "/Game/Input/InputActions/IA_Shoot.IA_Shoot"))
  (bind _bp_gun (Variables|Default|GetBP_Gun))
  ;[1 1 1] Fire
  (:Triggered
    (if (Variables|Default|GetbCanShoot)
      (Variables|Default|SetbCanShoot false)
      (Utilities|IsValid _bp_gun
        (:Is%20Valid
          (Default|Fire _bp_gun)
          (Utilities|FlowControl|Delay 0.2)
          (Variables|Default|SetbCanShoot true))))))

(event EventBeginPlay
  (bind _gun (Variables|Default|GetGun))
  (bind _gun_2 (Variables|Default|GetGun))
  (bind _lowerbody (Variables|Default|GetLowerBody))
  (bind _returnvalue (Transformation|GetWorldTransform _gun))
  (bind _asplayer_controller (Utilities|Casting|CastToPlayerController (Game|GetPlayerController 0)))
  (Utilities|IsValid (PlayerController|LocalPlayerSubsystems|GetEnhancedInputLocalPlayerSubsystem _asplayer_controller)
    (:Is%20Valid
      (Input|AddMappingContext (PlayerController|LocalPlayerSubsystems|GetEnhancedInputLocalPlayerSubsystem _asplayer_controller) "/Game/Input/IMC_DefaultInputMappingContext.IMC_DefaultInputMappingContext" 0 "(bIgnoreAllPressedKeysUntilRelease=True,bForceImmediately=False)")
      (Class|PrimitiveComponent|SetLinearDamping _lowerbody 0.5)
      (Class|PrimitiveComponent|SetAngularDamping _lowerbody 0.0)
      (Transformation|SetAbsolute (Variables|Default|GetGun) false true false)
      (bind _returnvalue_2 (Game|SpawnActorfromClass "/Game/_Game/Blueprints/Guns/BP_GunTest.BP_GunTest_C" (Math|Transform|MakeTransform (.location _returnvalue) (.rotation _returnvalue) "1.000000,1.000000,1.000000") "AdjustIfPossibleButAlwaysSpawn" 0 0))
      (bind _output_get (Variables|Default|SetBP_Gun _returnvalue_2))
      (Transformation|AttachComponentToComponent _output_get _gun_2 "None" "SnapToTarget" "KeepWorld" "KeepWorld" false)
      (Collision|SetCollisionEnabled _gun_2 "QueryAndPhysics"))))

(event EventTick
  (params (DeltaSeconds :type Float%20%28single-precision%29))
  (bind _force (CallFunction|GetMovementForceDirection))
  (bind _force_2 (CallFunction|GetMovementForceDirection))
  (bind _impactpoint (CallFunction|LineTraceforBodyRotation))
  (Transformation|SetWorldRotation (Variables|Default|GetGun) (Math|Rotator|MakeRotator 0.0 0.0 (.yaw (Math|Rotator|FindLookatRotation (Transformation|GetWorldLocation (Variables|Default|GetGun)) _impactpoint))) false false)
  (Transformation|SetWorldRotation (Variables|Default|GetUpperBody) (Math|Rotator|MakeRotator 0.0 0.0 (.yaw (Math|Rotator|FindLookatRotation (Transformation|GetWorldLocation (Variables|Default|GetGun)) _impactpoint))) false false)
  (if (Variables|Default|GetbMoveActionTriggered)
    ;[1 1 1] Movement Force and Turning Force
    (if (Variables|Default|GetbForceOverride)
      (Class|PrimitiveComponent|AddTorqueinRadians (Variables|Default|GetLowerBody) (Math|Vector|MakeVector (* (.y _force_2) -1.0) (.x _force_2) 0.0) "None" true)
      (else
        (Class|PrimitiveComponent|AddTorqueinRadians (Variables|Default|GetLowerBody) (Math|Vector|MakeVector (* (.y _force) -1.0) (.x _force) 0.0) "None" true)
        (Physics|AddForce (Variables|Default|GetLowerBody) (CallFunction|GetMovementTurnForce (CallFunction|GetMovementForceDirection)) "None" true)))))

(fn ConstructionScript)

(fn GetMovementForceDirection
  (bind _inputdirection (Variables|Default|GetInputDirection))
  (bind _moveforce (Variables|Default|GetMoveForce))
  (return (Math|Conversions|ToVector(Vector2D) (* (Math|Vector2D|MakeVector2D (* (.x _inputdirection) -1.0) (.y _inputdirection)) (Math|Vector2D|MakeVector2D _moveforce _moveforce)))))

(fn LineTraceforBodyRotation
  (bind _returnvalue (Game|GetPlayerController 0))
  (bind (_worldlocation _worlddirection) (Game|Player|ConvertMouseLocationToWorldSpace _returnvalue))
  (bind _outhit (Collision|LineTraceByChannel _worldlocation (+ _worldlocation (* _worlddirection 5e+03)) "TraceTypeQuery1" false 0 "None"))
  (return (.ImpactPoint (Collision|BreakHitResult _outhit))))

(fn GetMovementTurnForce
  (params (MovementForce :type Vector))
  (bind _returnvalue (Math|Vector|Normalize MovementForce))
  (bind _returnvalue_2 (Transformation|GetVelocity))
  (bind _returnvalue_3 (Math|Vector|Normalize _returnvalue_2))
  (return (* MovementForce (- 1.0 (+ (* (Math|Vector2D|DotProduct(2D) (Math|Vector2D|MakeVector2D (.x _returnvalue) (.y _returnvalue)) (Math|Vector2D|MakeVector2D (.x _returnvalue_3) (.y _returnvalue_3))) 0.5) 0.5)) (Variables|Default|GetTurnForce))))