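; BP_Missile is a missile launcher weapon that fires missile projectiles.
; Its Fire event spawns a scaled-down BP_MissileProjectile at the location and rotation of Barrel1, adjusting around collisions but always spawning.
; The graph holds no other active logic: BeginPlay, overlap and Tick are disabled stubs, and the construction script only calls its parent.
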(event EventBeginPlay
  (|CallParentFunction) ; This node is disabled and will not be called.\nDrag off pins to build functionality.
)

(event Collision|EventActorBeginOverlap
  (params (OtherActor :type Actor%20Object%20Reference))
  (|CallParentFunction OtherActor) ; This node is disabled and will not be called.\nDrag off pins to build functionality.
)

(event EventTick
  (params (DeltaSeconds :type Float%20%28single-precision%29))
  (|CallParentFunction DeltaSeconds) ; This node is disabled and will not be called.\nDrag off pins to build functionality.
)

(event EventFire
  (bind _barrel_1 (Variables|Default|GetBarrel_1))
  (bind _returnvalue (Transformation|GetWorldTransform _barrel_1))
  (Game|SpawnActorfromClass "/Game/_Game/Blueprints/Projectiles/BP_MissileProjectile.BP_MissileProjectile_C" (Math|Transform|MakeTransform (.location _returnvalue) (.rotation _returnvalue) "0.400000,0.400000,0.400000") "AdjustIfPossibleButAlwaysSpawn" 0 0))

(fn ConstructionScript
  (|CallParentFunction))